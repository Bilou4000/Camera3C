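; Player controller for a 3D strategy camera that pans, zooms, orbits and centers on interactive components.
; Enhanced Input moves the BP_Camera pawn along its arrow, sets a clamped desired arm length, and rotates the spring arm with clamped pitch, yawing the arrow to match.
; While not interacting, Tick sphere-traces along camera forward for "interactive"-tagged components; clicking eases the pawn to the hit component.
; BDTCamera supplies the tuning values.
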(event Input|EnhancedActionEvents|EnhancedInputActionIA_Zoom
  (params (ActionValue :type Float%20%28double-precision%29) (ElapsedSeconds :type Float%20%28double-precision%29) (TriggeredSeconds :type Float%20%28double-precision%29) (InputAction :type Input%20Action%20Object%20Reference :default "/Game/Claire/Input/IA_Zoom.IA_Zoom"))
  (bind _bdt_camera (Variables|Reference|GetBDT_Camera))
  ;[1 1 1] ZoomCamera
  (Variables|/Game/Claire/_GameManager/BP_Camera.BP_Camera_C|SetdesireArmLenght (Variables|Reference|GetAs%20BP%20Camera) (Math|Float|Clamp(Float) (+ (Variables|/Game/Claire/_GameManager/BP_Camera.BP_Camera_C|GetdesireArmLenght (Variables|Reference|GetAs%20BP%20Camera)) (* (* ActionValue -1.0) (Variables|/Game/Claire/DataAsset/BDT_Camera.BDT_Camera_C|GetzoomInputStep (Variables|Reference|GetBDT_Camera)))) (Variables|/Game/Claire/DataAsset/BDT_Camera.BDT_Camera_C|GetminZoom _bdt_camera) (Variables|/Game/Claire/DataAsset/BDT_Camera.BDT_Camera_C|GetmaxZoom _bdt_camera))))

(event Input|EnhancedActionEvents|EnhancedInputActionIA_MoveCamera
  (params (ActionValue :type Vector%202D%20Structure) (ElapsedSeconds :type Float%20%28double-precision%29) (TriggeredSeconds :type Float%20%28double-precision%29) (InputAction :type Input%20Action%20Object%20Reference :default "/Game/Claire/Input/IA_MoveCamera.IA_MoveCamera"))
  (bind _bdt_camera (Variables|Reference|GetBDT_Camera))
  (bind _as_bp_camera (Variables|Reference|GetAs%20BP%20Camera))
  (bind _as_bp_camera_2 (Variables|Reference|GetAs%20BP%20Camera))
  ;[1 1 1] MoveCamera
  (Pawn|Input|AddMovementInput _as_bp_camera_2 (Math|Vector|GetRightVector (Variables|/Game/Claire/_GameManager/BP_Camera.BP_Camera_C|GetArrow _as_bp_camera_2)) (* (.x ActionValue) (Variables|/Game/Claire/DataAsset/BDT_Camera.BDT_Camera_C|GetsideSpeed _bdt_camera)) false)
  (Pawn|Input|AddMovementInput _as_bp_camera (Math|Vector|GetForwardVector (Variables|/Game/Claire/_GameManager/BP_Camera.BP_Camera_C|GetArrow _as_bp_camera)) (* (.y ActionValue) (Variables|/Game/Claire/DataAsset/BDT_Camera.BDT_Camera_C|GetforwardSpeed _bdt_camera)) false))

(event Input|EnhancedActionEvents|EnhancedInputActionIA_OnClick
  (params (ActionValue :type Boolean) (ElapsedSeconds :type Float%20%28double-precision%29) (TriggeredSeconds :type Float%20%28double-precision%29) (InputAction :type Input%20Action%20Object%20Reference :default "/Game/Claire/Input/IA_OnClick.IA_OnClick"))
  (:Triggered
    (if (Variables|Bool|GetcanInteract)
      (Variables|Bool|SetisInteracting true)
      (Components|MoveComponentTo (Variables|/Script/Engine.Actor|GetRootComponent (Variables|Reference|GetAs%20BP%20Camera)) (Variables|/Script/Engine.SceneComponent|GetRelativeLocation (Variables|Default|GetHit%20Component)) "0, 0, 0" false true (Variables|/Game/Claire/DataAsset/BDT_Camera.BDT_Camera_C|GetcenterToCharacterSpeed (Variables|Reference|GetBDT_Camera)) false)
      (else
        (Variables|Bool|SetisInteracting false)))))

(event Input|EnhancedActionEvents|EnhancedInputActionIA_GyroscopeCamera
  (params (ActionValue :type Vector%202D%20Structure) (ElapsedSeconds :type Float%20%28double-precision%29) (TriggeredSeconds :type Float%20%28double-precision%29) (InputAction :type Input%20Action%20Object%20Reference :default "/Game/Claire/Input/IA_GyroscopeCamera.IA_GyroscopeCamera"))
  (bind _as_bp_camera (Variables|Reference|GetAs%20BP%20Camera))
  (bind _as_bp_camera_2 (Variables|Reference|GetAs%20BP%20Camera))
  (bind _as_bp_camera_3 (Variables|Reference|GetAs%20BP%20Camera))
  (bind _bdt_camera (Variables|Reference|GetBDT_Camera))
  (bind _springarm (Variables|/Game/Claire/_GameManager/BP_Camera.BP_Camera_C|GetSpringArm _as_bp_camera_2))
  (bind _springarm_2 (Variables|/Game/Claire/_GameManager/BP_Camera.BP_Camera_C|GetSpringArm _as_bp_camera_3))
  (bind _returnvalue (Transformation|GetWorldRotation _springarm_2))
  (bind _returnvalue_2 (Transformation|GetWorldRotation _springarm))
  ;[1 1 1] Rotate Camera
  (Variables|Default|SetAction%20Value%20X (.x ActionValue))
  (Variables|Default|SetAction%20Value%20Y (.y ActionValue))
  ;;[0.05788 0.1379 1] Rotate Camera on Z Axis
  (Transformation|SetWorldRotation (Variables|/Game/Claire/_GameManager/BP_Camera.BP_Camera_C|GetSpringArm (Variables|Reference|GetAs%20BP%20Camera)) (Math|Rotator|MakeRotator (.roll _returnvalue_2) (.pitch _returnvalue_2) (+ (.yaw _returnvalue_2) (* (Variables|Default|GetAction%20Value%20X) (Variables|/Game/Claire/DataAsset/BDT_Camera.BDT_Camera_C|GetspeedGyroscope (Variables|Reference|GetBDT_Camera))))) false false)
  ;;[0.2157 1 0.2198] Rotate Camera on Y Axis
  (Transformation|SetWorldRotation (Variables|/Game/Claire/_GameManager/BP_Camera.BP_Camera_C|GetSpringArm (Variables|Reference|GetAs%20BP%20Camera)) (Math|Rotator|MakeRotator (.roll _returnvalue) (Math|Float|Clamp(Float) (+ (.pitch _returnvalue) (* (Variables|Default|GetAction%20Value%20Y) (Variables|/Game/Claire/DataAsset/BDT_Camera.BDT_Camera_C|GetspeedGyroscope (Variables|Reference|GetBDT_Camera)))) (Variables|/Game/Claire/DataAsset/BDT_Camera.BDT_Camera_C|GetminYRotation _bdt_camera) (Variables|/Game/Claire/DataAsset/BDT_Camera.BDT_Camera_C|GetmaxYRotation _bdt_camera)) (.yaw _returnvalue)) false false)
  ;;[1 0.1453 0.1354] Rotate Arrow on Z Axis considering spring arm rotation
  (Transformation|SetWorldRotation (Variables|/Game/Claire/_GameManager/BP_Camera.BP_Camera_C|GetArrow _as_bp_camera) (Math|Rotator|MakeRotator 0.0 0.0 (.yaw (Transformation|GetWorldRotation (Variables|/Game/Claire/_GameManager/BP_Camera.BP_Camera_C|GetSpringArm _as_bp_camera)))) false false))

(event EventBeginPlay
  (bind _returnvalue (PlayerController|LocalPlayerSubsystems|GetEnhancedInputLocalPlayerSubsystem))
  ;[1 1 1] Begin Play
  (bind _asbp_camera (Utilities|Casting|CastToBP_Camera (Game|Player|GetPlayerPawn 0)))
  (Variables|Reference|SetAs%20BP%20Camera _asbp_camera)
  (Utilities|IsValid _returnvalue
    (:Is%20Valid
      (Input|AddMappingContext _returnvalue "/Game/Claire/Input/IC_3DStrategy.IC_3DStrategy" 0 "(bIgnoreAllPressedKeysUntilRelease=True,bForceImmediately=False,bNotifyUserSettings=False)"))))

(event EventTick
  (params (DeltaSeconds :type Float%20%28single-precision%29))
  (bind _as_bp_camera (Variables|Reference|GetAs%20BP%20Camera))
  (bind _camera (Variables|/Game/Claire/_GameManager/BP_Camera.BP_Camera_C|GetCamera _as_bp_camera))
  (bind _returnvalue (Transformation|GetWorldLocation _camera))
  (if (not (Variables|Bool|GetisInteracting))
    ;[1 1 1] Convert Center of screen pos to world
    (bind _outhit (Collision|SphereTraceByChannel _returnvalue (+ _returnvalue (* (Math|Vector|GetForwardVector (Transformation|GetWorldRotation _camera)) (Variables|/Game/Claire/DataAsset/BDT_Camera.BDT_Camera_C|GetraycastLenght (Variables|Reference|GetBDT_Camera)))) 2e+01 "TraceTypeQuery1" false 0 "None"))
    (Utilities|IsValid (.HitComponent (Collision|BreakHitResult _outhit))
      (:Is%20Valid
        (if (Components|ComponentHasTag (.HitComponent (Collision|BreakHitResult _outhit)) "interactive")
          (Variables|Bool|SetcanInteract true)
          (Variables|Default|SetHit%20Component (.HitComponent (Collision|BreakHitResult _outhit)))
          (else
            (Variables|Bool|SetcanInteract false)))))))

(fn ConstructionScript)