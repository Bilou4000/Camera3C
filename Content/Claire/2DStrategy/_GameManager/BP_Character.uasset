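; BP_Character is a character Blueprint in the 2D strategy game that smooths the zoom of its orthographic camera.
; BeginPlay seeds DesiredOrthoWidth from the camera's current width.
; Each Tick lerps the camera's OrthoWidth toward that target by delta time times BDT2DTopDown's ZoomSmoothSpeed, giving an eased zoom.
; Nothing in these graphs changes the target after startup.
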(event EventBeginPlay
  ;[1 1 1] Begin Play
  (Variables|Default|SetdesiredOrthoWidth (Variables|/Script/Engine.CameraComponent|GetOrthoWidth (Variables|Default|GetCamera))))

(event EventTick
  (params (DeltaSeconds :type Float%20%28single-precision%29))
  ;[1 1 1] Event Tick
  (Variables|/Script/Engine.CameraComponent|SetOrthoWidth (Variables|Default|GetCamera) (Math|Float|Lerp (Variables|/Script/Engine.CameraComponent|GetOrthoWidth (Variables|Default|GetCamera)) (Variables|Default|GetdesiredOrthoWidth) (* DeltaSeconds (Variables|/Game/Claire/2DStrategy/DataAsset/BDT_2DTopDown.BDT_2DTopDown_C|GetzoomSmoothSpeed (Variables|Default|GetBDT_2DTopDown))))))

(fn ConstructionScript)