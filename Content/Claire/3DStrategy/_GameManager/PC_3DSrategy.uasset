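; Player controller for the 3D strategy mode, driving a BP_Camera pawn through Enhanced Input with tuning from BDT3DStrategy.
; Move, zoom and rotate inputs are clamped where needed, with an Arrow following spring arm yaw to keep movement horizontal.
; Tick sphere-traces along the camera's view for "interactive"-tagged components; clicking toggles centering on one, which pauses movement and tracing.
; Another input opens the 3D TopDown level.
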(event Input|EnhancedActionEvents|EnhancedInputActionIA_Zoom
  (params (ActionValue :type Float%20%28double-precision%29) (ElapsedSeconds :type Float%20%28double-precision%29) (TriggeredSeconds :type Float%20%28double-precision%29) (InputAction :type Input%20Action%20Object%20Reference :default "/Game/Claire/3DStrategy/Input/IA_Zoom.IA_Zoom"))
  (bind _bdt_3dstrategy (Variables|Reference|GetBDT_3DStrategy))
  ;[1 1 1] ZoomCamera
  (Variables|/Game/Claire/3DStrategy/_GameManager/BP_Camera.BP_Camera_C|SetdesireArmLenght (Variables|Reference|GetAs%20BP%20Camera) (Math|Float|Clamp(Float) (+ (Variables|/Game/Claire/3DStrategy/_GameManager/BP_Camera.BP_Camera_C|GetdesireArmLenght (Variables|Reference|GetAs%20BP%20Camera)) (* (* ActionValue -1.0) (Variables|/Game/Claire/3DStrategy/DataAsset/BDT_3DStrategy.BDT_3DStrategy_C|GetzoomInputStep (Variables|Reference|GetBDT_3DStrategy)))) (Variables|/Game/Claire/3DStrategy/DataAsset/BDT_3DStrategy.BDT_3DStrategy_C|GetminZoom _bdt_3dstrategy) (Variables|/Game/Claire/3DStrategy/DataAsset/BDT_3DStrategy.BDT_3DStrategy_C|GetmaxZoom _bdt_3dstrategy))))

(event Input|EnhancedActionEvents|EnhancedInputActionIA_MoveCamera
  (params (ActionValue :type Vector%202D%20Structure) (ElapsedSeconds :type Float%20%28double-precision%29) (TriggeredSeconds :type Float%20%28double-precision%29) (InputAction :type Input%20Action%20Object%20Reference :default "/Game/Claire/3DStrategy/Input/IA_MoveCamera.IA_MoveCamera"))
  (bind _as_bp_camera (Variables|Reference|GetAs%20BP%20Camera))
  (bind _as_bp_camera_2 (Variables|Reference|GetAs%20BP%20Camera))
  ;[1 1 1] MoveCamera
  (if (not (Variables|Bool|GetisInteracting))
    (Pawn|Input|AddMovementInput _as_bp_camera_2 (Math|Vector|GetRightVector (Variables|/Game/Claire/3DStrategy/_GameManager/BP_Camera.BP_Camera_C|GetArrow _as_bp_camera_2)) (.x ActionValue) false)
    (Pawn|Input|AddMovementInput _as_bp_camera (Math|Vector|GetForwardVector (Variables|/Game/Claire/3DStrategy/_GameManager/BP_Camera.BP_Camera_C|GetArrow _as_bp_camera)) (.y ActionValue) false)))

(event Input|EnhancedActionEvents|EnhancedInputActionIA_OnClick
  (params (ActionValue :type Boolean) (ElapsedSeconds :type Float%20%28double-precision%29) (TriggeredSeconds :type Float%20%28double-precision%29) (InputAction :type Input%20Action%20Object%20Reference :default "/Game/Claire/3DStrategy/Input/IA_OnClick.IA_OnClick"))
  ;[1 1 1] Click On Object
  (:Started
    (if (Variables|Bool|GetcanInteract)
      (Utilities|FlowControl|FlipFlop
        (:A
          (Variables|Bool|SetisInteracting true)
          (Components|MoveComponentTo (Variables|/Script/Engine.Actor|GetRootComponent (Variables|Reference|GetAs%20BP%20Camera)) (Variables|/Script/Engine.SceneComponent|GetRelativeLocation (Variables|Default|GetHit%20Component)) "0, 0, 0" false true (Variables|/Game/Claire/3DStrategy/DataAsset/BDT_3DStrategy.BDT_3DStrategy_C|GetcenterToCharacterSpeed (Variables|Reference|GetBDT_3DStrategy)) false))
        (:B
          (Variables|Bool|SetisInteracting false :!label _label)))
      (else
        (goto _label)))))

(event Input|EnhancedActionEvents|EnhancedInputActionIA_GyroscopeCamera
  (params (ActionValue :type Vector%202D%20Structure) (ElapsedSeconds :type Float%20%28double-precision%29) (TriggeredSeconds :type Float%20%28double-precision%29) (InputAction :type Input%20Action%20Object%20Reference :default "/Game/Claire/3DStrategy/Input/IA_GyroscopeCamera.IA_GyroscopeCamera"))
  (bind _as_bp_camera (Variables|Reference|GetAs%20BP%20Camera))
  (bind _as_bp_camera_2 (Variables|Reference|GetAs%20BP%20Camera))
  (bind _as_bp_camera_3 (Variables|Reference|GetAs%20BP%20Camera))
  (bind _bdt_3dstrategy (Variables|Reference|GetBDT_3DStrategy))
  (bind _springarm (Variables|/Game/Claire/3DStrategy/_GameManager/BP_Camera.BP_Camera_C|GetSpringArm _as_bp_camera_2))
  (bind _springarm_2 (Variables|/Game/Claire/3DStrategy/_GameManager/BP_Camera.BP_Camera_C|GetSpringArm _as_bp_camera_3))
  (bind _returnvalue (Transformation|GetWorldRotation _springarm_2))
  (bind _returnvalue_2 (Transformation|GetWorldRotation _springarm))
  ;[1 1 1] Rotate Camera
  (Variables|CameraMovement|SetRotateX (.x ActionValue))
  (Variables|CameraMovement|SetRotateY (.y ActionValue))
  ;;[0.05788 0.1379 1] Rotate Camera on Z Axis
  (Transformation|SetWorldRotation (Variables|/Game/Claire/3DStrategy/_GameManager/BP_Camera.BP_Camera_C|GetSpringArm (Variables|Reference|GetAs%20BP%20Camera)) (Math|Rotator|MakeRotator (.roll _returnvalue_2) (.pitch _returnvalue_2) (+ (.yaw _returnvalue_2) (* (Variables|CameraMovement|GetRotateX) (Variables|/Game/Claire/3DStrategy/DataAsset/BDT_3DStrategy.BDT_3DStrategy_C|GetspeedGyroscope (Variables|Reference|GetBDT_3DStrategy))))) false false)
  ;;[0.2157 1 0.2198] Rotate Camera on Y Axis
  (Transformation|SetWorldRotation (Variables|/Game/Claire/3DStrategy/_GameManager/BP_Camera.BP_Camera_C|GetSpringArm (Variables|Reference|GetAs%20BP%20Camera)) (Math|Rotator|MakeRotator (.roll _returnvalue) (Math|Float|Clamp(Float) (+ (.pitch _returnvalue) (* (Variables|CameraMovement|GetRotateY) (Variables|/Game/Claire/3DStrategy/DataAsset/BDT_3DStrategy.BDT_3DStrategy_C|GetspeedGyroscope (Variables|Reference|GetBDT_3DStrategy)))) (Variables|/Game/Claire/3DStrategy/DataAsset/BDT_3DStrategy.BDT_3DStrategy_C|GetminYRotation _bdt_3dstrategy) (Variables|/Game/Claire/3DStrategy/DataAsset/BDT_3DStrategy.BDT_3DStrategy_C|GetmaxYRotation _bdt_3dstrategy)) (.yaw _returnvalue)) false false)
  ;;[1 0.1453 0.1354] Rotate Arrow on Z Axis considering spring arm rotation
  (Transformation|SetWorldRotation (Variables|/Game/Claire/3DStrategy/_GameManager/BP_Camera.BP_Camera_C|GetArrow _as_bp_camera) (Math|Rotator|MakeRotator 0.0 0.0 (.yaw (Transformation|GetWorldRotation (Variables|/Game/Claire/3DStrategy/_GameManager/BP_Camera.BP_Camera_C|GetSpringArm _as_bp_camera)))) false false))

(event Input|EnhancedActionEvents|EnhancedInputActionIA_SwitchTo3DTopDown
  (params (ActionValue :type Boolean) (ElapsedSeconds :type Float%20%28double-precision%29) (TriggeredSeconds :type Float%20%28double-precision%29) (InputAction :type Input%20Action%20Object%20Reference :default "/Game/Claire/3DStrategy/Input/IA_SwitchTo3DTopDown.IA_SwitchTo3DTopDown"))
  ;[1 1 1] Switch to next level (3D TopDown)
  (Game|OpenLevel(byObjectReference) "/Game/Omid-Folder/Level/Asset_3DTopDown.Asset_3DTopDown"))

(event EventBeginPlay
  (bind _returnvalue (PlayerController|LocalPlayerSubsystems|GetEnhancedInputLocalPlayerSubsystem))
  ;[1 1 1] Begin Play
  (bind _asbp_camera (Utilities|Casting|CastToBP_Camera (Game|Player|GetPlayerPawn 0)))
  (Variables|Reference|SetAs%20BP%20Camera _asbp_camera)
  (Utilities|IsValid _returnvalue
    (:Is%20Valid
      (Input|AddMappingContext _returnvalue "/Game/Claire/3DStrategy/Input/IC_3DStrategy.IC_3DStrategy" 0 "(bIgnoreAllPressedKeysUntilRelease=True,bForceImmediately=False,bNotifyUserSettings=False)")
      (Variables|/Script/Engine.FloatingPawnMovement|SetMaxSpeed (Variables|/Game/Claire/3DStrategy/_GameManager/BP_Camera.BP_Camera_C|GetFloatingPawnMovement (Variables|Reference|GetAs%20BP%20Camera)) (* (Variables|/Game/Claire/3DStrategy/DataAsset/BDT_3DStrategy.BDT_3DStrategy_C|GetmoveSpeed (Variables|Reference|GetBDT_3DStrategy)) 1e+01)))))

(event EventTick
  (params (DeltaSeconds :type Float%20%28single-precision%29))
  (bind _as_bp_camera (Variables|Reference|GetAs%20BP%20Camera))
  (bind _camera (Variables|/Game/Claire/3DStrategy/_GameManager/BP_Camera.BP_Camera_C|GetCamera _as_bp_camera))
  (bind _returnvalue (Transformation|GetWorldLocation _camera))
  ;[1 1 1] Event Tick
  (if (not (Variables|Bool|GetisInteracting))
    ;;[1 0.7135 0.2207] Convert Center of screen pos to world
    (bind _outhit (Collision|SphereTraceByChannel _returnvalue (+ _returnvalue (* (Math|Vector|GetForwardVector (Transformation|GetWorldRotation _camera)) (Variables|/Game/Claire/3DStrategy/DataAsset/BDT_3DStrategy.BDT_3DStrategy_C|GetraycastLenght (Variables|Reference|GetBDT_3DStrategy)))) 2e+01 "TraceTypeQuery1" false 0 "None"))
    ;;[0.2404 0.3951 1] Check if you can interract with component
    (Utilities|IsValid (.HitComponent (Collision|BreakHitResult _outhit))
      (:Is%20Valid
        (if (Components|ComponentHasTag (.HitComponent (Collision|BreakHitResult _outhit)) "interactive")
          (Variables|Bool|SetcanInteract true)
          (Variables|Default|SetHit%20Component (.HitComponent (Collision|BreakHitResult _outhit)))
          (else
            (Variables|Bool|SetcanInteract false)))))))

(fn ConstructionScript)