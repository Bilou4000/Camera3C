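; BP_Camera is the camera Blueprint for the 3D strategy game, providing smoothed zoom through its spring arm.
; On BeginPlay it stores the spring arm's current length as the desired length.
; Each tick it lerps the arm length toward that desired value, with alpha scaled by delta time and the zoom smoothing speed from BDT3DStrategy.
; Nothing in its graphs changes the desired length after initialization.
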(event EventBeginPlay
  ;[1 1 1] Begin Play
  (Variables|Default|SetdesireArmLenght (Variables|/Script/Engine.SpringArmComponent|GetTargetArmLength (Variables|Default|GetSpringArm))))

(event EventTick
  (params (DeltaSeconds :type Float%20%28single-precision%29))
  ;[1 1 1] Event Tick
  (Variables|/Script/Engine.SpringArmComponent|SetTargetArmLength (Variables|Default|GetSpringArm) (Math|Float|Lerp (Variables|/Script/Engine.SpringArmComponent|GetTargetArmLength (Variables|Default|GetSpringArm)) (Variables|Default|GetdesireArmLenght) (* DeltaSeconds (Variables|/Game/Claire/3DStrategy/DataAsset/BDT_3DStrategy.BDT_3DStrategy_C|GetzoomSmoothSpeed (Variables|Default|GetBDT_3DStrategy))))))

(fn ConstructionScript)