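; BP_PlayerController is a player controller that rotates the top-down character's camera boom around the vertical axis on player input.
; On BeginPlay it casts the player pawn to BP_TopDownCharacter and caches the reference.
; The IA_Rotate Enhanced Input action uses the sign of its value to step the SpringArm's world yaw by plus or minus RotationAngle, forcing pitch and roll to zero.
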(event Input|EnhancedActionEvents|EnhancedInputActionIA_Rotate
  (params (ActionValue :type Float%20%28double-precision%29) (ElapsedSeconds :type Float%20%28double-precision%29) (TriggeredSeconds :type Float%20%28double-precision%29) (InputAction :type Input%20Action%20Object%20Reference :default "/Game/Omid-Folder/Inputs/IA_Rotate.IA_Rotate"))
  (bind _bp_topdowncharacter (Variables|Default|GetBP_TopDownCharacter))
  (bind _bp_topdowncharacter_2 (Variables|Default|GetBP_TopDownCharacter))
  (bind _springarm (Variables|/Game/Omid-Folder/Blueprints/BP_TopDownCharacter.BP_TopDownCharacter_C|GetSpringArm _bp_topdowncharacter))
  (bind _springarm_2 (Variables|/Game/Omid-Folder/Blueprints/BP_TopDownCharacter.BP_TopDownCharacter_C|GetSpringArm _bp_topdowncharacter_2))
  (if (> ActionValue 0.0)
    (Transformation|SetWorldRotation _springarm_2 (Math|Rotator|MakeRotator 0.0 0.0 (+ (.yaw (Transformation|GetWorldRotation _springarm_2)) (Variables|Default|GetRotation%20angle))) false false)
    (elif (< ActionValue 0.0)
      (Transformation|SetWorldRotation _springarm (Math|Rotator|MakeRotator 0.0 0.0 (+ (.yaw (Transformation|GetWorldRotation _springarm)) (* (Variables|Default|GetRotation%20angle) -1.0))) false false))))

(event EventBeginPlay
  (bind _asbp_top_down_character (Utilities|Casting|CastToBP_TopDownCharacter (Game|Player|GetPlayerPawn 0)))
  (Variables|Default|SetBP_TopDownCharacter _asbp_top_down_character))

(fn ConstructionScript)